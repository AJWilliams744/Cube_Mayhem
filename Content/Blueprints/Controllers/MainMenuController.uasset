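; MainMenuController is a main menu controller that turns input actions into menu commands.
; On BeginPlay it casts the game mode to MainMenu_GM and stores the reference.
; D-pad up and down presses step the menu value by plus or minus one, while Select and Back call their matching game mode functions, leaving all menu logic to the game mode.
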(event `self.ReceiveBeginPlay`
  (bind _asmain_menu_gm (cast `/Game/Blueprints/GameModes/MainMenu_GM` (`GameplayStatics.GetGameMode`)))
  (set `self.GM` _asmain_menu_gm))

(event `InputAction|DPadDown`
  (params (Key :type "Key Structure"))
  (:`Pressed`
    (`/Game/Blueprints/GameModes/MainMenu_GM.UpdateMenuValue` (`self.GM`) -1)))

(event `InputAction|DPadUp`
  (params (Key :type "Key Structure"))
  (:`Pressed`
    (`/Game/Blueprints/GameModes/MainMenu_GM.UpdateMenuValue` (`self.GM`) 1)))

(event `InputAction|Select`
  (params (Key :type "Key Structure"))
  (:`Pressed`
    (`/Game/Blueprints/GameModes/MainMenu_GM.SelectMenu` (`self.GM`))))

(event `InputAction|Back`
  (params (Key :type "Key Structure"))
  (:`Pressed`
    (`/Game/Blueprints/GameModes/MainMenu_GM.Back` (`self.GM`))))

(fn `UserConstructionScript`)