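; Player hero character for a bullet-hell shooter, with axis-driven movement and aiming, gun fire and a big area blast.
; A BasicGun spawned at GunSocket handles normal and alternate fire, and holding fire slows walking.
; BigFire damages IDamagable pawns in a sphere after a delay, with a timer cooldown shown through body material glow.
; Pause, menu input and death are forwarded to BulletHell_GM.
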(event `InputAxis|MoveRight`
  (params (AxisValue :type "Float (single-precision)"))
  ;[1 1 1] Movement
  (`self.AddMovementInput` (0.0 1.0 0.0) AxisValue))

(event `InputAxis|LookUp`
  (params (AxisValue :type "Float (single-precision)"))
  ;[1 1 1] Shooting
  (bind _returnvalue (`KismetMathLibrary.MakeVector` AxisValue (stale `InputAxis|LookRight` AxisValue)))
  (if (> (`KismetMathLibrary.VSize` _returnvalue) 0.4) :!label _label
    (`Controller.SetControlRotation` (`self.GetController`) (`KismetMathLibrary.MakeRotFromX` _returnvalue))))

(event `InputAction|Fire`
  (params (Key :type "Key Structure"))
  (bind _basicwepon (`self.BasicWepon`))
  ;[1 1 1] Fire
  (:`Pressed`
    (if (`self.AllowedNormalFire`)
      (`/Game/Blueprints/Gun_Bulets/BasicGun_BP.PullTrigger` _basicwepon)
      (set `CharacterMovementComponent.MaxWalkSpeed` (`self.SlowSpeed`) (`self.CharacterMovement`))))
  (:`Released`
    (`/Game/Blueprints/Gun_Bulets/BasicGun_BP.ReleaseTrigger` _basicwepon)
    (set `CharacterMovementComponent.MaxWalkSpeed` (`self.Speed`) (`self.CharacterMovement`))))

(event `InputAxis|LookRight`
  (params (AxisValue :type "Float (single-precision)"))
  ;[1 1 1] Shooting
  (goto _label))

(event `InputAxis|MoveUp`
  (params (AxisValue :type "Float (single-precision)"))
  ;[1 1 1] Movement
  (`self.AddMovementInput` (1.0 0.0 0.0) AxisValue))

(event `InputAction|AlternateFire`
  (params (Key :type "Key Structure"))
  ;[1 1 1] Fire
  (:`Pressed`
    (if (`self.AllowedAlternateFire`)
      (`/Game/Blueprints/Gun_Bulets/BasicGun_BP.AlternateFire` (`self.BasicWepon`)))))

(event `InputAction|BigFire`
  (params (Key :type "Key Structure"))
  (bind _returnvalue (/ 1.0 (`self.BigFireRate`)))
  ;[1 1 1] Fire
  (:`Pressed`
    (if (`self.CanUseBigFire`)
      (set `self.CanUseBigFire` false)
      (`KismetSystemLibrary.K2_SetTimer` null "BigFireReset" _returnvalue false _returnvalue)
      (`MaterialInstanceDynamic.SetScalarParameterValue` (`self.BodyDynamicMat`) "GlowMultiplier" 0.0)
      (`GameplayStatics.PlaySoundAtLocation` "/Game/Sounds/393374__eflexmusic__big-sci-fi-explosion-bomb-close-mixed.393374__eflexmusic__big-sci-fi-explosion-bomb-close-mixed" (`self.K2_GetActorLocation`) (struct) 1.0 1.0 0.0 null null null)
      (`KismetSystemLibrary.Delay` 1.0)
      (`self.HandleBigFire`)
      (`GameplayStatics.SpawnEmitterAttached` "/Game/ParticleSystem/HeroBigGun.HeroBigGun" (`self.CapsuleComponent`)))))

(event `BigFireReset`
  ;[1 1 1] Fire
  (set `self.CanUseBigFire` true)
  (`KismetSystemLibrary.K2_ClearTimer` null "BigFireReset")
  (`MaterialInstanceDynamic.SetScalarParameterValue` (`self.BodyDynamicMat`) "GlowMultiplier" 0.5)
  (`GameplayStatics.PlaySound2D` "/Game/Sounds/BigLaserCharge.BigLaserCharge" 1.0 1.0 0.0 null null))

(event `InputAction|Back`
  (params (Key :type "Key Structure"))
  (:`Pressed`
    (`/Game/Blueprints/GameModes/BulletHell_GM.BackPressed` (`self.GM`))))

(event `InputAction|Select`
  (params (Key :type "Key Structure"))
  (:`Pressed`
    (`/Game/Blueprints/GameModes/BulletHell_GM.SelectPressed` (`self.GM`))))

(event `self.ReceiveBeginPlay`
  ;[1 1 1] Begin Play
  (`parent.ReceiveBeginPlay`)
  (bind _returnvalue (`|SpawnActorFromClass` "/Game/Blueprints/Gun_Bulets/BasicGun_BP.BasicGun_BP_C" (`SceneComponent.K2_GetComponentToWorld` (`self.GunSocket`)) "AlwaysSpawn" "OverrideRootScale" null null))
  (bind _output_get (set `self.BasicWepon` _returnvalue))
  (`self.K2_AttachToComponent` _output_get (`self.GunSocket`) "None" "KeepWorld" "KeepWorld" "KeepWorld" true)
  (bind _asbullet_hell_gm (cast `/Game/Blueprints/GameModes/BulletHell_GM` (`GameplayStatics.GetGameMode`)))
  (set `self.GM` _asbullet_hell_gm))

(event `Key|Gamepad_Special_Right` :paused true
  (params (Key :type "Key Structure"))
  (bind _gm (`self.GM`))
  (:`Pressed`
    (if (`GameplayStatics.IsGamePaused`)
      (`GameplayStatics.SetGamePaused` false)
      (`/Game/Blueprints/Gun_Bulets/BasicGun_BP.ReleaseTrigger` (`self.BasicWepon`))
      (`/Game/Blueprints/GameModes/BulletHell_GM.PausedRemoved` _gm)
      (set `CharacterMovementComponent.MaxWalkSpeed` (`self.Speed`) (`self.CharacterMovement`))
      (else
        (`GameplayStatics.SetGamePaused` true)
        (`/Game/Blueprints/GameModes/BulletHell_GM.PausedPressed` _gm)))))

(event `Key|Gamepad_FaceButton_Bottom` :paused true
  (params (Key :type "Key Structure"))
  (:`Pressed`
    (`/Game/Blueprints/GameModes/BulletHell_GM.SelectPressed` (`self.GM`))))

(event `/Game/Blueprints/iDamagable.AffectHealth`
  (params (DamageAmount :type "Float (single-precision)") (ByGun :type Boolean) (BulletRotation :type "Rotator Structure") (ByPassDeath :type Boolean))
  ;[1 1 1] Affect Health
  (bind _output_get (set `self.Health` (- (`self.Health`) DamageAmount)))
  (bind _output_get_2 (set `self.IsDead` (<= _output_get 0.0)))
  (if _output_get_2
    (`/Engine/EditorBlueprintResources/StandardMacros.DoOnce` false
      (:`Completed`
        (`/Game/Blueprints/GameModes/BulletHell_GM.OnPlayerDeath` (`self.GM`) null)))))

(fn `HandleBigFire`
  (bind _outactors (`KismetSystemLibrary.SphereOverlapActors` (`self.K2_GetActorLocation`) 1500.0 (`|MakeArray` "ObjectTypeQuery3" :!type "EObjectTypeQuery Enum") null (`|MakeArray` self :!type "Actor Object Reference")))
  (for _array_element _outactors
    (if (`KismetSystemLibrary.DoesImplementInterface` _array_element "/Game/Blueprints/iDamagable.iDamagable_C")
      (message `/Game/Blueprints/iDamagable.AffectHealth` _array_element 1500.0 true (`KismetMathLibrary.MakeRotFromX` (- (`self.K2_GetActorLocation` _array_element) (`self.K2_GetActorLocation`))) true))))

(fn `UserConstructionScript`
  (`parent.UserConstructionScript`)
  (bind _returnvalue (`PrimitiveComponent.CreateDynamicMaterialInstance` (`self.Head`) 0 null "None"))
  (bind _output_get (set `self.HeadDynamicMat` _returnvalue))
  (`MaterialInstanceDynamic.SetScalarParameterValue` _output_get "GlowMultiplier" 0.1)
  (bind _returnvalue_2 (`PrimitiveComponent.CreateDynamicMaterialInstance` (`self.Body`) 0 null "None"))
  (bind _output_get_2 (set `self.BodyDynamicMat` _returnvalue_2))
  (`MaterialInstanceDynamic.SetScalarParameterValue` _output_get_2 "GlowMultiplier" 0.1)
  (`MaterialInstanceDynamic.SetVectorParameterValue` _output_get_2 "BaseColour" (struct :`R` 0.648265 :`G` 1.0 :`A` 1.0)))