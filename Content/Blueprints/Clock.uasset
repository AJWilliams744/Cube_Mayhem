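; Bullet-hell clock actor whose rotating arm advances game stages as it enters each of four yaw quadrants.
; Tick steps MainRotator behind a short Delay, and GetRotationArea maps its yaw to a sector.
; Chained, mutually resetting DoOnces recolour the directional light and the dynamic material shared by all static meshes, then call TriggerNextStage on BulletHell_GM.
; TriggerSector flashes supplied pillars but is not called here.
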(event `self.ReceiveTick`
  (params (DeltaSeconds :type "Float (single-precision)"))
  (bind _dynamicmat (`self.DynamicMat`))
  (bind (_returnvalue_roll _returnvalue_pitch _returnvalue_yaw) (`KismetMathLibrary.BreakRotator` (`SceneComponent.K2_GetComponentRotation` (`self.MainRotator`))))
  (bind _lightcomponent (`Light.LightComponent` (`self.DirectionalLight`)))
  (`KismetSystemLibrary.Delay` 0.2)
  (`SceneComponent.K2_AddWorldRotation` (`self.MainRotator`) (`KismetMathLibrary.MakeRotator` 0.0 0.0 (* DeltaSeconds (`self.Speed`))) false false)
  (bind _sector (`self.GetRotationArea` _returnvalue_yaw))
  (switch `int` _sector
    (:`0`
      (`|ExecutionSequence`
        (:`then_0`
          (`/Engine/EditorBlueprintResources/StandardMacros.DoOnce` false :!label _label
            (:`Completed`
              (`MaterialInstanceDynamic.SetVectorParameterValue` _dynamicmat "Colour" (struct :`G` 0.286154 :`B` 1.0 :`A` 1.0))
              (`LightComponent.SetLightColor` _lightcomponent (struct :`G` 0.287441 :`B` 1.0 :`A` 1.0) true)
              (`|ExecutionSequence`
                (:`then_0`
                  _)
                (:`then_1`
                  (goto _label_4 :!via `Reset`))))))
        (:`then_1`
          (goto _label_4 :!via `Reset`))))
    (:`1`
      (`/Engine/EditorBlueprintResources/StandardMacros.DoOnce` false :!label _label_2
        (:`Completed`
          (`MaterialInstanceDynamic.SetVectorParameterValue` _dynamicmat "Colour" (struct :`R` 1.0 :`G` 0.893594 :`A` 1.0))
          (`LightComponent.SetLightColor` _lightcomponent (struct :`R` 1.0 :`G` 0.896269 :`A` 1.0) true)
          (`|ExecutionSequence`
            (:`then_0`
              _)
            (:`then_1`
              (goto _label :!via `Reset`))))))
    (:`2`
      (`/Engine/EditorBlueprintResources/StandardMacros.DoOnce` false :!label _label_3
        (:`Completed`
          (`MaterialInstanceDynamic.SetVectorParameterValue` _dynamicmat "Colour" (struct :`R` 1.0 :`B` 0.763201 :`A` 1.0))
          (`LightComponent.SetLightColor` _lightcomponent (struct :`R` 1.0 :`B` 0.768151 :`A` 1.0) true)
          (`|ExecutionSequence`
            (:`then_0`
              _)
            (:`then_1`
              (goto _label_2 :!via `Reset`))))))
    (:`3`
      (`/Engine/EditorBlueprintResources/StandardMacros.DoOnce` true :!label _label_4
        (:`Completed`
          (`MaterialInstanceDynamic.SetVectorParameterValue` _dynamicmat "Colour" (struct :`R` 1.0 :`A` 1.0))
          (`LightComponent.SetLightColor` _lightcomponent (struct :`R` 0.693872 :`A` 1.0) true)
          (`|ExecutionSequence`
            (:`then_0`
              _)
            (:`then_1`
              (goto _label_3 :!via `Reset`)))))))
  (bind _asbullet_hell_gm (cast `/Game/Blueprints/GameModes/BulletHell_GM` (`GameplayStatics.GetGameMode`)))
  (`/Game/Blueprints/GameModes/BulletHell_GM.TriggerNextStage` _asbullet_hell_gm))

(fn `GetRotationArea`
  (params (Rotation :type "Float (double-precision)"))
  (returns (Sector :type Integer))
  (locals (LocalSector :type Integer))
  (if (or (> Rotation 135.0) (< Rotation -135.0))
    (set `local.LocalSector` 2)
    (return (`local.LocalSector`))
    (elif (or (and (> Rotation 0.0) (< Rotation 45.0)) (and (> Rotation -45.0) (< Rotation 0.0)))
      (set `local.LocalSector` 0)
      (return (`local.LocalSector`))
      (elif (and (> Rotation 45.0) (< Rotation 135.0))
        (set `local.LocalSector` 1)
        (return (`local.LocalSector`))
        (elif (and (> Rotation -135.0) (< Rotation -45.0))
          (set `local.LocalSector` 3)
          (return (`local.LocalSector`)))))))

(fn `TriggerSector`
  (params (SectorPillar :type "Array of /Game/Blueprints/Pillar Object Reference"))
  (for _array_element SectorPillar
    (`/Game/Blueprints/Pillar.TriggerFlashingLight` _array_element)))

(fn `UserConstructionScript`
  (bind _returnvalue (`PrimitiveComponent.CreateDynamicMaterialInstance` (`self.ClockArm`) 0 null "None"))
  (set `self.DynamicMat` _returnvalue)
  (for _array_element (`self.K2_GetComponentsByClass` "/Script/Engine.StaticMeshComponent")
    (`PrimitiveComponent.SetMaterial` _array_element 0 (`self.DynamicMat`))))