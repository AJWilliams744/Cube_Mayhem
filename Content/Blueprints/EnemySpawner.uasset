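; Enemy spawner Blueprint that repeatedly spawns an AI pawn of the EnemyVarient1 class inside a box area.
; StartSpawning sets a looping timer on SpawnEnemy at an interval of one over SpawnRate, and StopSpawning clears it.
; Each spawn picks a random point within the scaled extent of SpawnArea.
; Nothing runs on BeginPlay or Tick, so spawning begins only when StartSpawning is called.
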(event `SpawnEnemy`
  (bind _spawnarea (`self.SpawnArea`))
  (`AIBlueprintHelperLibrary.SpawnAIFromClass` "/Game/Blueprints/EnemyVarient1.EnemyVarient1_C" null (`KismetMathLibrary.RandomPointInBoundingBox` (`SceneComponent.K2_GetComponentLocation` _spawnarea) (`BoxComponent.GetScaledBoxExtent` _spawnarea)) (struct) false null))

(event `StartSpawning`
  (`KismetSystemLibrary.K2_SetTimer` null "SpawnEnemy" (/ 1.0 (`self.SpawnRate`)) true))

(event `StopSpawning`
  (`KismetSystemLibrary.K2_ClearTimer` null "SpawnEnemy"))

(fn `UserConstructionScript`)