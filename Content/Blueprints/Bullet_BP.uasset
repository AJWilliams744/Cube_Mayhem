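; Projectile bullet actor that deals damage when its collision sphere hits an actor implementing IDamagable, then destroys itself.
; Such hits send an AffectHealth interface message with a big-gun flag and play a sound and particle effect; other hits are ignored.
; Optional splash damage messages damagable pawns within a radius, excluding the player, dividing damage by the splash percentage fraction.
; The construction script tints the sphere through a dynamic material instance.
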(event `self.ReceiveBeginPlay`
  (add `self.OnDestroyed` (delegate `Destroy`)))

(event `Destroy` :!signature `self.OnDestroyed`
  (params (DestroyedActor :type "Actor Object Reference"))
  (`self.Destroyed`))

(event `Destroyed`)

(event `self.Sphere1.OnComponentHit`
  (params (HitComponent :type "PrimitiveComponent Object Reference") (OtherActor :type "Actor Object Reference") (OtherComp :type "PrimitiveComponent Object Reference") (NormalImpulse :type "Vector Structure") (Hit :type "HitResult Structure (by ref)"))
  (bind (_bblockinghit _binitialoverlap _time _distance _location _impactpoint _normal _impactnormal) (`GameplayStatics.BreakHitResult` Hit))
  (bind (_returnvalue_roll _returnvalue_pitch _returnvalue_yaw) (`KismetMathLibrary.BreakRotator` (`self.K2_GetActorRotation`)))
  (if (`KismetSystemLibrary.DoesImplementInterface` OtherActor "/Game/Blueprints/iDamagable.iDamagable_C")
    (message `/Game/Blueprints/iDamagable.AffectHealth` OtherActor (`self.Damage`) (`self.AmIABigGun`))
    (`GameplayStatics.PlaySoundAtLocation` (`self.Sound`) (`SceneComponent.K2_GetComponentLocation` (`self.Sphere`)) (struct) 1.0 1.0 0.0 null null null)
    (`GameplayStatics.SpawnEmitterAtLocation` (`self.EmitterHit`) (+ _impactpoint (* _impactnormal 1.0)) (`KismetMathLibrary.MakeRotator` _returnvalue_yaw 90.0) (0.1 0.1 0.1))
    (if (`self.DoesSplashDamage`)
      (bind (_outactors _returnvalue) (`KismetSystemLibrary.SphereOverlapActors` (`SceneComponent.K2_GetComponentLocation` (`self.Sphere`)) (`self.SplashSize`) (`|MakeArray` "ObjectTypeQuery3" :!type "EObjectTypeQuery Enum") null (`|MakeArray` (`GameplayStatics.GetPlayerCharacter` 0) :!type "Actor Object Reference")))
      (if _returnvalue
        (for _array_element _outactors
          (if (`KismetSystemLibrary.DoesImplementInterface` _array_element "/Game/Blueprints/iDamagable.iDamagable_C")
            (message `/Game/Blueprints/iDamagable.AffectHealth` _array_element (/ (`self.Damage`) (/ (`self.SpashPercentage`) 100.0)) (`self.AmIABigGun`))))))
    (`self.K2_DestroyActor`)))

(fn `UserConstructionScript`
  (bind _returnvalue (`PrimitiveComponent.CreateDynamicMaterialInstance` (`self.Sphere`) 0 null "None"))
  (bind _output_get (set `self.DynamicMat` _returnvalue))
  (`MaterialInstanceDynamic.SetVectorParameterValue` _output_get "Colour" (`self.BulletColour`)))