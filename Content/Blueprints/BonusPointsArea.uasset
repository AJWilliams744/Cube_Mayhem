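; BonusPointsArea is a bullet-hell bonus zone actor tied to a PointCaster.
; It ends when the PointCaster is destroyed or when a looping timer finds the player over 850 units away.
; Either path stores the caster's Count times Multiplier as BonusPoints, then plays a sound and particle burst, resets the GameMode multiplier to 1 and destroys the area.
; BonusPoints is only stored here, not added to a score.
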(event `self.ReceiveBeginPlay`
  (add `self.OnDestroyed` (`self.PointCaster`) (delegate `Destroyed`))
  (`KismetSystemLibrary.K2_SetTimer` null "CheckDistance" 0.5 true))

(event `Destroyed` :!signature `self.OnDestroyed`
  (params (DestroyedActor :type "Actor Object Reference"))
  (bind _returnvalue (`self.K2_GetActorLocation`))
  (bind _aspoint_hinter (cast `/Game/Blueprints/PointHinter` DestroyedActor))
  (set `self.BonusPoints` (* (`/Game/Blueprints/PointHinter.Multiplier` _aspoint_hinter) (`/Game/Blueprints/PointHinter.Count` _aspoint_hinter)))
  (`GameplayStatics.PlaySoundAtLocation` "/Game/Sounds/ReverseBang.ReverseBang" _returnvalue (struct) 4.0 1.0 1.0 null null null :!label _label)
  (`GameplayStatics.SpawnEmitterAtLocation` "/Game/ParticleSystem/MagicCircleDestroyed.MagicCircleDestroyed" _returnvalue)
  (bind _asbullet_hell_gm (cast `/Game/Blueprints/GameModes/BulletHell_GM` (`GameplayStatics.GetGameMode`)))
  (set `/Game/Blueprints/GameModes/BulletHell_GM.Multiplier` 1 _asbullet_hell_gm)
  (`self.K2_DestroyActor`))

(event `CheckDistance`
  (bind _pointcaster (`self.PointCaster`))
  (if (> (`KismetMathLibrary.Vector_Distance` (`self.K2_GetActorLocation`) (`self.K2_GetActorLocation` (`GameplayStatics.GetPlayerCharacter` 0))) 850.0)
    (set `self.BonusPoints` (* (`/Game/Blueprints/PointHinter.Count` _pointcaster) (`/Game/Blueprints/PointHinter.Multiplier` _pointcaster)))
    (goto _label)))

(fn `UserConstructionScript`)