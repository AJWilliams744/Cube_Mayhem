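; Game mode for the main menu that loads saved data and shows the menu widget.
; On BeginPlay it calls LoadGame on the game instance, adds a MainMenu widget to the viewport, hides the cursor and sets game-only input.
; Its navigation, select and back events forward to the widget, so the menu is driven through the game mode rather than by mouse.
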(event `self.ReceiveBeginPlay`
  (bind _asthe_game_instance (cast `/Game/Blueprints/TheGameInstance` (`GameplayStatics.GetGameInstance`)))
  (`/Game/Blueprints/TheGameInstance.LoadGame` _asthe_game_instance)
  (bind _returnvalue (`|CreateWidget` "/Game/WidgetBlueprints/MainMenu.MainMenu_C"))
  (bind _output_get (set `self.Hud` _returnvalue))
  (`UserWidget.AddToViewport` _output_get 0)
  (set `PlayerController.bShowMouseCursor` false (`GameplayStatics.GetPlayerController` 0))
  (`WidgetBlueprintLibrary.SetInputMode_GameOnly` (`GameplayStatics.GetPlayerController` 0)))

(event `UpdateMenuValue`
  (params (Direction :type Integer))
  (`/Game/WidgetBlueprints/MainMenu.UpdateMenuValue` (`self.Hud`) Direction))

(event `SelectMenu`
  (`/Game/WidgetBlueprints/MainMenu.SelectMenu` (`self.Hud`)))

(event `Back`
  (`/Game/WidgetBlueprints/MainMenu.BackPressed` (`self.Hud`)))

(fn `UserConstructionScript`)