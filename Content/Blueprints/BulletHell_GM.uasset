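; Bullet-hell game mode that creates the HUD, starts all enemy spawners and manages score and multiplier.
; AddScore adds multiplied points and raises the multiplier whenever the score sum meets the threshold, which stays met because BaseScore never resets.
; A clamped timer, shorter at very high multipliers, decays the multiplier toward one.
; Score popups update the last PointHinter if near the player, otherwise spawn another; the player-death handler is empty.
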(event `self.ReceiveBeginPlay`
  (`|ExecutionSequence`
    (:`then_0`
      (bind _returnvalue (`|CreateWidget` "/Game/WidgetBlueprints/HUD_Widget.HUD_Widget_C"))
      (bind _output_get (set `self.Hud` _returnvalue))
      (`UserWidget.AddToViewport` _output_get 0)
      (bind _outactors (`GameplayStatics.GetAllActorsOfClass` "/Game/Blueprints/EnemySpawner.EnemySpawner_C"))
      (for _array_element _outactors
        (`/Game/Blueprints/EnemySpawner.StartSpawning` _array_element)))
    (:`then_1`
      (add `self.OnDestroyed` (`GameplayStatics.GetPlayerCharacter` 0) (delegate `OnPlayerDeath`)))))

(event `ReduceMultiplier`
  ;[1 1 1] Reduce Multiplier
  (if (not (== (`self.Multiplier`) 1))
    (`/Engine/EditorBlueprintResources/StandardMacros.DecrementInt` (`self.Multiplier`)
      (:`  `
        (`self.ResetMultiplierTimer`)))))

(event `OnPlayerDeath` :!signature `self.OnDestroyed`
  (params (DestroyedActor :type "Actor Object Reference")))

(event `AddScore`
  (params (Points :type Integer))
  (bind _basescore (`self.BaseScore`))
  (bind _multiplier (`self.Multiplier`))
  ;[1 1 1] Add Score
  (`self.ResetMultiplierTimer`)
  (`self.FirePointHelper` Points _multiplier)
  (set `self.BaseScore` (+ (* Points _multiplier) _basescore))
  (if (>= (+ _basescore (`self.MultiplierScore`)) (`self.ScoreForMultiplierIncrease`))
    (set `self.MultiplierScore` 0)
    (`/Engine/EditorBlueprintResources/StandardMacros.IncrementInt` (`self.Multiplier`))))

(event `FirePointHelper`
  (params (Points :type Integer) (Multiplier :type Integer))
  (bind _returnvalue (`SceneComponent.K2_GetComponentLocation` (`Character.CapsuleComponent` (`GameplayStatics.GetPlayerCharacter` 0))))
  ;[1 1 1] Fire Score Indicator
  (bind _scoreshower (`self.ScoreShower`)
    (:`then`
      (if (<= (`KismetMathLibrary.Vector_Distance` (`SceneComponent.K2_GetComponentLocation` (`/Game/Blueprints/PointHinter.DefaultSceneRoot` _scoreshower)) _returnvalue) 150.0)
        (`/Game/Blueprints/PointHinter.UpdateValues` _scoreshower Points Multiplier)
        (else
          (bind _returnvalue_2 (`|SpawnActorFromClass` "/Game/Blueprints/PointHinter.PointHinter_C" (`KismetMathLibrary.MakeTransform` _returnvalue) "Undefined" "OverrideRootScale" null Points Multiplier null :!label _label))
          (set `self.ScoreShower` _returnvalue_2))))
    (:`else`
      (goto _label))))

(fn `ResetMultiplierTimer`
  (`KismetSystemLibrary.K2_SetTimer` null "ReduceMultiplier" (`KismetMathLibrary.FClamp` (`KismetMathLibrary.Conv_IntToDouble` (- 50 (`self.Multiplier`))) 0.1 5.0) true))

(fn `UserConstructionScript`)