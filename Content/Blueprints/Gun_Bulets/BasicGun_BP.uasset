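; BasicGun_BP is a laser gun with automatic primary fire and a heavier alternate shot on a cooldown.
; Holding the trigger fires immediately, then repeats on a looping timer, spawning Bullet_BP with sound and force feedback.
; Alternate fire spawns BigBullet_BP with stronger feedback and camera shake, dimming the HeroCharacter's head glow until a reset timer restores it.
; A dynamic material shows each shot's colour, with a timeline driving the brightness flare.
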(event `PullTrigger`
  (`/Engine/EditorBlueprintResources/StandardMacros.DoOnce` false :!label _label
    (:`Completed`
      (`self.Fire`)
      (`KismetSystemLibrary.K2_SetTimer` null "Fire" (/ 1.0 (`self.Firerate`)) true))))

(event `ReleaseTrigger`
  (`KismetSystemLibrary.K2_ClearTimer` null "Fire")
  (goto _label :!via `Reset`))

(event `Fire`
  (bind _forcefeedback (`self.ForceFeedback`))
  (`MaterialInstanceDynamic.SetVectorParameterValue` (`self.GunMat`) "Colour" (`self.Colour`))
  (`|SpawnActorFromClass` "/Game/Blueprints/Gun_Bulets/Bullet_BP.Bullet_BP_C" (`SceneComponent.K2_GetComponentToWorld` (`self.ProjectileSpawn`)) "AlwaysSpawn" "OverrideRootScale" null (`self.BulletDamage`) (`self.Colour`) null)
  (`GameplayStatics.PlaySoundAtLocation` "/Game/Sounds/LaserGun.LaserGun" (`SceneComponent.K2_GetComponentLocation` (`self.ProjectileSpawn`)) (struct) 0.6 1.0 0.0 null null null)
  (set `ForceFeedbackComponent.IntensityMultiplier` 0.1 _forcefeedback)
  (`ForceFeedbackComponent.Play` _forcefeedback 0.0)
  (bind (_direction _delta) (`Timeline|FlareUp` :!via `PlayFromStart` :!label _label_2)
    (:`Update`
      (`MaterialInstanceDynamic.SetScalarParameterValue` (`self.GunMat`) "Brightness" _delta))))

(event `AlternateFire`
  (bind _forcefeedback (`self.ForceFeedback`))
  (bind _returnvalue (/ 1.0 (`self.AlternateFireRate`)))
  (if (`self.AlternateCanFire`)
    (set `self.AlternateCanFire` false)
    (`KismetSystemLibrary.K2_SetTimer` null "WeponReset" _returnvalue false _returnvalue)
    (`self.SetHeadGlow` 0.0)
    (`MaterialInstanceDynamic.SetVectorParameterValue` (`self.GunMat`) "Colour" (`self.AlterateColour`))
    (`|SpawnActorFromClass` "/Game/Blueprints/Gun_Bulets/BigBullet_BP.BigBullet_BP_C" (`SceneComponent.K2_GetComponentToWorld` (`self.ProjectileSpawn`)) "AlwaysSpawn" "OverrideRootScale" null (`self.AlternateBulletDamage`) (`self.AlterateColour`) null)
    (`GameplayStatics.PlaySoundAtLocation` "/Game/Sounds/BigLaserGun.BigLaserGun" (`SceneComponent.K2_GetComponentLocation` (`self.ProjectileSpawn`)) (struct) 1.4 1.0 0.0 null null null)
    (`PlayerController.ClientStartCameraShake` :`self` (`GameplayStatics.GetPlayerController` 0) :`Shake` "/Game/Blueprints/CameraShake1.CameraShake1_C" :`Scale` 0.2)
    (set `ForceFeedbackComponent.IntensityMultiplier` 5.0 _forcefeedback)
    (`ForceFeedbackComponent.Play` _forcefeedback 0.0)
    (goto _label_2 :!via `PlayFromStart`)))

(event `WeponReset`
  (set `self.AlternateCanFire` true)
  (`KismetSystemLibrary.K2_ClearTimer` null "WeponReset")
  (`self.SetHeadGlow` 0.1)
  (`GameplayStatics.PlaySound2D` "/Game/Sounds/SmallLaserCharge.SmallLaserCharge" 1.0 1.0 0.0 null null))

(fn `SetHeadGlow`
  (params (Value :type "Float (double-precision)"))
  (bind _ashero_character (cast `/Game/Blueprints/HeroCharacter` (`GameplayStatics.GetPlayerCharacter` 0)))
  (`MaterialInstanceDynamic.SetScalarParameterValue` (`/Game/Blueprints/HeroCharacter.HeadDynamicMat` _ashero_character) "GlowMultiplier" Value)
  (return))

(fn `UserConstructionScript`
  (bind _returnvalue (`PrimitiveComponent.CreateDynamicMaterialInstance` (`self.Gun`) 0 null "None"))
  (set `self.GunMat` _returnvalue))