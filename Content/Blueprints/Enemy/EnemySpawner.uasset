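; Enemy spawner that periodically creates EnemyVarient1 AI at random points inside its SpawnArea box, up to a MaxEnemys cap.
; Start and stop events drive a looping SpawnEnemy timer whose interval comes from SpawnRate.
; Each spawn receives the spawner's stats and material colour, and its destruction decrements the live count.
; IncrementSpeed scales the stored slow and max speeds that later spawns inherit.
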(event `SpawnEnemy`
  (bind _spawnarea (`self.SpawnArea`))
  (if (not (>= (`self.TotalEnemys`) (`self.MaxEnemys`)))
    (`/Engine/EditorBlueprintResources/StandardMacros.IncrementInt` (`self.TotalEnemys`)
      (:`  `
        (bind _returnvalue (`AIBlueprintHelperLibrary.SpawnAIFromClass` "/Game/Blueprints/Enemy/EnemyVarient1.EnemyVarient1_C" null (`KismetMathLibrary.RandomPointInBoundingBox` (`SceneComponent.K2_GetComponentLocation` _spawnarea) (`BoxComponent.GetScaledBoxExtent` _spawnarea)) (struct) false null))
        (bind _asenemy_varient_1 (cast `/Game/Blueprints/Enemy/EnemyVarient1` _returnvalue))
        (set `/Game/Blueprints/Enemy/EnemyVarient1.DamageRad` (`self.SplashRange`) _asenemy_varient_1)
        (set `/Game/Blueprints/Enemy/EnemyVarient1.SlowSpeed` (`self.EnemySlowSpeed`) _asenemy_varient_1)
        (set `/Game/Blueprints/BaseCharacter_BP.Speed` (`self.EnemyMaxSpeed`) _asenemy_varient_1)
        (set `/Game/Blueprints/BaseCharacter_BP.MaxHealth` (`self.EnemyHealth`) _asenemy_varient_1)
        (set `/Game/Blueprints/Enemy/EnemyVarient1.HitDamage` (`self.HitDamage`) _asenemy_varient_1)
        (`/Game/Blueprints/Enemy/EnemyVarient1.UpdateValues` _asenemy_varient_1)
        (`MaterialInstanceDynamic.SetVectorParameterValue` (`/Game/Blueprints/Enemy/EnemyVarient1.DynamicMaterial` _asenemy_varient_1) "MainColour" (`self.EnemyColour`))
        (add `self.OnDestroyed` _asenemy_varient_1 (delegate `ReduceCount`))))))

(event `StartSpawning`
  (`KismetSystemLibrary.K2_SetTimer` null "SpawnEnemy" (/ 1.0 (`self.SpawnRate`)) true))

(event `IncrementSpeed`
  (set `self.EnemySlowSpeed` (* (`self.EnemySlowSpeed`) 1.2))
  (set `self.EnemyMaxSpeed` (* (`self.EnemyMaxSpeed`) 1.2)))

(event `ReduceCount` :!signature `self.OnDestroyed`
  (params (DestroyedActor :type "Actor Object Reference"))
  (`/Engine/EditorBlueprintResources/StandardMacros.DecrementInt` (`self.TotalEnemys`)))

(event `StopSpawning`
  (`KismetSystemLibrary.K2_ClearTimer` null "SpawnEnemy"))

(fn `UserConstructionScript`)