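; Main menu game mode that puts the MainMenu widget on screen and sets up input for it.
; On BeginPlay it creates and stores the widget, shows the mouse cursor and sets Game and UI input with focus on the Play button.
; An UpdateMenu event relays a direction to the widget's UpdateMenuValue.
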(event `self.ReceiveBeginPlay`
  (bind _returnvalue (`|CreateWidget` "/Game/WidgetBlueprints/MainMenu.MainMenu_C"))
  (bind _output_get (set `self.Hud` _returnvalue))
  (`UserWidget.AddToViewport` _output_get 0)
  (set `PlayerController.bShowMouseCursor` true (`GameplayStatics.GetPlayerController` 0))
  (`WidgetBlueprintLibrary.SetInputMode_GameAndUIEx` (`GameplayStatics.GetPlayerController` 0) (`/Game/WidgetBlueprints/MainMenu.PlayButton` (`self.Hud`))))

(event `UpdateMenu`
  (params (Direction :type Integer))
  (`/Game/WidgetBlueprints/MainMenu.UpdateMenuValue` (`self.Hud`) Direction))

(fn `UserConstructionScript`)