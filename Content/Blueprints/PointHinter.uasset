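; PointHinter is a short-lived actor that shows a points popup as animated text.
; On BeginPlay it sets its text and plays a timeline that drives the text's X and Y scale, then destroys itself when the animation finishes.
; UpdateValues adds to the running count, replaces the multiplier, shows both as "Points X Multiplier", sets a fixed base scale and restarts the animation, extending the popup's life.
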(event `self.ReceiveBeginPlay`
  (bind _points (`self.Points`))
  (`TextRenderComponent.K2_SetText` _points (`self.Text`))
  (bind (_direction _scale) (`Timeline|Animation` :!via `PlayFromStart` :!label _label)
    (:`Update`
      (bind _returnvalue (* _scale (`self.BaseScale`)))
      (`TextRenderComponent.SetXScale` _points _returnvalue)
      (`TextRenderComponent.SetYScale` _points _returnvalue))
    (:`Finished`
      (`self.K2_DestroyActor`))))

(event `UpdateValues`
  (params (AdditionalCount :type Integer) (NewMultiplier :type Integer))
  (set `self.BaseScale` 2.0)
  (set `self.Count` (+ AdditionalCount (`self.Count`)))
  (set `self.Multiplier` NewMultiplier)
  (`TextRenderComponent.K2_SetText` (`self.Points`) (`|FormatText` "{Points} X {Multiplier}" (`self.Count`) (`self.Multiplier`)))
  (goto _label :!via `PlayFromStart`))

(fn `UserConstructionScript`)