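; Cube enemy variant for a bullet-hell game that explodes on death and kills itself on contact with the hero, damaging them.
; Hits briefly slow it and update a dynamic material's damage colour from health.
; Death plays a scale timeline, then particles, sound and camera shake before destroying the actor.
; Unless bypassed, the blast damages nearby pawns, hurts the player with linear distance falloff and awards score through the game mode.
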(event `HitVariables`
  (`self.UpdateColourFromHealth`)
  (set `CharacterMovementComponent.MaxWalkSpeed` (`self.SlowSpeed`) (`self.CharacterMovement`))
  (`KismetSystemLibrary.K2_SetTimer` null "ResetSlowSpeed" 0.5 false 0.5))

(event `self.AffectHealth`
  (params (DamageAmount :type "Float (single-precision)") (ByGun :type Boolean) (BulletRotation :type "Rotator Structure") (ByPassDeath :type Boolean))
  ;[1 1 1] Affect Health
  (set `self.HitByGun` ByGun)
  (if (not (`self.IsDead`))
    (set `self.BulletRotation` BulletRotation)
    (set `self.ByPassDeath` ByPassDeath)
    (`self.HitVariables`)
    (bind _output_get (set `self.Health` (- (`self.Health`) DamageAmount)))
    (bind _output_get_2 (set `self.IsDead` (<= _output_get 0.0)))
    (if _output_get_2
      (`self.OnDeath`))))

(event `self.ReceiveBeginPlay`
  (`parent.ReceiveBeginPlay`)
  (`self.UpdateColourFromHealth`))

(event `ResetSlowSpeed`
  (set `CharacterMovementComponent.MaxWalkSpeed` (`self.Speed`) (`self.CharacterMovement`))
  (`KismetSystemLibrary.K2_ClearTimer` null "ResetSlowSpeed"))

(event `OnDeath`
  (bind (_bulletrotation_roll _bulletrotation_pitch _bulletrotation_yaw) (`KismetMathLibrary.BreakRotator` (`self.BulletRotation`)))
  (bind _returnvalue (`SceneComponent.K2_GetComponentLocation` (`self.Cube`)))
  ;[1 1 1] On Death
  (`/Engine/EditorBlueprintResources/StandardMacros.DoOnce` false
    (:`Completed`
      (if (`self.HitByGun`)
        (set `self.DeathParticle` "/Game/ParticleSystem/CubeDeathHit.CubeDeathHit")
        (else
          (set `self.DeathParticle` "/Game/ParticleSystem/CubeDeath.CubeDeath")))
      (`PrimitiveComponent.SetCollisionResponseToChannel` (`self.CapsuleComponent`) "ECC_Pawn" "ECR_Ignore")
      (if (not (`self.ByPassDeath`))
        (bind (_direction _scale) (`Timeline|DeathAnim`)
          (:`Update`
            (`SceneComponent.SetWorldScale3D` (`self.Cube`) (`KismetMathLibrary.MakeVector` _scale _scale _scale)))
          (:`Finished`
            (`GameplayStatics.SpawnEmitterAtLocation` (`self.DeathParticle`) _returnvalue (`KismetMathLibrary.MakeRotator` 0.0 0.0 (- _bulletrotation_yaw 180.0)) :!label _label)
            (`GameplayStatics.PlaySoundAtLocation` "/Game/Sounds/CubeDeath.CubeDeath" _returnvalue (struct) 1.0 1.0 0.0 null null null)
            (`PlayerController.ClientStartCameraShake` :`self` (`GameplayStatics.GetPlayerController` 0) :`Shake` "/Game/CameraShake1.CameraShake1_C")
            (if (not (`self.ByPassDeath`))
              (`self.HandleHits`))
            (`self.K2_DestroyActor`)))
        (else
          (goto _label))))))

(event `self.CapsuleComponent.OnComponentHit`
  (params (HitComponent :type "PrimitiveComponent Object Reference") (OtherActor :type "Actor Object Reference") (OtherComp :type "PrimitiveComponent Object Reference") (NormalImpulse :type "Vector Structure") (Hit :type "HitResult Structure (by ref)"))
  ;[1 1 1] On Hit
  (bind _ashero_character (cast `/Game/Blueprints/HeroCharacter` OtherActor))
  (`/Engine/EditorBlueprintResources/StandardMacros.DoOnce` false
    (:`Completed`
      (`self.AffectHealth` 1000.0)
      (`self.AffectHealth` :`self` _ashero_character :`DamageAmount` (`self.HitDamage`)))))

(fn `DamageRadius`
  (params (Radius :type "Float (double-precision)") (Damage :type "Float (double-precision)"))
  (locals (NewLocalVar_0 :type "Actor Object Reference"))
  (bind (_outactors _returnvalue) (`KismetSystemLibrary.SphereOverlapActors` (`SceneComponent.K2_GetComponentLocation` (`self.CapsuleComponent`)) Radius (`|MakeArray` "ObjectTypeQuery3" :!type "EObjectTypeQuery Enum") null (`|MakeArray` self (`GameplayStatics.GetPlayerCharacter` 0) :!type "Actor Object Reference")))
  (if _returnvalue
    (for _array_element _outactors
      (message `/Game/Blueprints/iDamagable.AffectHealth` _array_element Damage false (struct) false))
    (return)))

(fn `HandleHits`
  (bind _returnvalue (`GameplayStatics.GetPlayerCharacter` 0))
  (bind _splashrange (`self.SplashRange`))
  (bind _returnvalue_2 (`KismetMathLibrary.Vector_Distance` (`SceneComponent.K2_GetComponentLocation` (`self.CapsuleComponent`)) (`SceneComponent.K2_GetComponentLocation` (`Character.Mesh` _returnvalue))))
  (`self.DamageRadius` 100.0 40.0)
  (if (`KismetMathLibrary.InRange_FloatFloat` _returnvalue_2 0.0 _splashrange)
    (message `/Game/Blueprints/iDamagable.AffectHealth` _returnvalue (/ (- _splashrange _returnvalue_2) (`self.SplashDivider`)) false (struct) false)
    (if (not (`/Game/Blueprints/BaseCharacter_BP.IsDead` (cast `/Game/Blueprints/HeroCharacter` (`GameplayStatics.GetPlayerCharacter` 0) :!pure true)))
      (`/Game/Blueprints/BulletHell_GM.AddScore` (cast `/Game/Blueprints/BulletHell_GM` (`GameplayStatics.GetGameMode`) :!pure true) (`self.Points`) :!label _label))
    (else
      (goto _label))))

(fn `UpdateColourFromHealth`
  (`MaterialInstanceDynamic.SetScalarParameterValue` (`self.DynamicMaterial`) "Damage" (* (/ (`self.Health`) (`self.MaxHealth`)) 2.0)))

(fn `UserConstructionScript`
  (`parent.UserConstructionScript`)
  (bind _returnvalue (`PrimitiveComponent.CreateDynamicMaterialInstance` (`self.Cube`) 0 null "None"))
  (set `self.DynamicMaterial` _returnvalue))